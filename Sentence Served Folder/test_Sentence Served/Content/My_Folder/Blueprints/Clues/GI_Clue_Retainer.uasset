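; Game Instance for clue retention that picks the level's murder weapon actor for the mystery.
; Getweapon switches on the stored murder weapon type and stores a random actor carrying the matching size/shape tag as MurderWeapon.
; As a debug aid, it prints the chosen actor's name and, after a short delay, spawns a RectLight at its transform.
; Nested DoOnce gates limit selection; WeaponChooseReset resets only the inner one.
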(event `Get weapon`
  (bind _murderweapon (`self.MurderWeapon`))
  (`/Engine/EditorBlueprintResources/StandardMacros.DoOnce` false
    (:`Completed`
      (bind _asgi_clue_retainer (cast `/Game/My_Folder/Blueprints/Clues/GI_Clue_Retainer` (`GameplayStatics.GetGameInstance`)))
      (`/Engine/EditorBlueprintResources/StandardMacros.DoOnce` false :!label _label
        (:`Completed`
          (switch `int` (`/Game/My_Folder/Blueprints/Clues/GI_Clue_Retainer.GI_MurderWeaponType` _asgi_clue_retainer)
            (:`0`
              (bind _outactors (`GameplayStatics.GetAllActorsWithTag` "Large Blunt"))
              (set `self.MurderWeapon` (`KismetArrayLibrary.Array_Random` _outactors)))
            (:`1`
              (bind _outactors_2 (`GameplayStatics.GetAllActorsWithTag` "Small Blunt"))
              (set `self.MurderWeapon` (`KismetArrayLibrary.Array_Random` _outactors_2)))
            (:`2`
              (bind _outactors_3 (`GameplayStatics.GetAllActorsWithTag` "Miscellaneous"))
              (set `self.MurderWeapon` (`KismetArrayLibrary.Array_Random` _outactors_3)))
            (:`3`
              (bind _outactors_4 (`GameplayStatics.GetAllActorsWithTag` "Large Sharp"))
              (set `self.MurderWeapon` (`KismetArrayLibrary.Array_Random` _outactors_4)))
            (:`4`
              (bind _outactors_5 (`GameplayStatics.GetAllActorsWithTag` "Small Sharp"))
              (set `self.MurderWeapon` (`KismetArrayLibrary.Array_Random` _outactors_5))))
          ;[1 0.6174 0.15 0.5] Find object debug
          (`KismetSystemLibrary.PrintString` (`KismetSystemLibrary.GetDisplayName` _murderweapon))
          (`KismetSystemLibrary.Delay` 1.0)
          (`|SpawnActorFromClass` "/Script/Engine.RectLight" (`Actor.GetTransform` _murderweapon) "AdjustIfPossibleButAlwaysSpawn" "MultiplyWithRoot" null null))))))

(event `Weapon Choose Reset`
  (goto _label :!via `Reset`))